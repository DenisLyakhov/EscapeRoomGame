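; Interactable door Blueprint that starts opening or closing on interaction once unlocked, and otherwise has the player open an inventory message.
; Applying an item with CanOpenLock after an interaction unlocks it, shows the unlocked message, closes the inventory message and triggers the door immediately.
; A FlipFlop alternates playing and reversing a timeline that lerps the mesh's yaw through a 90-degree swing.
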(event `/Game/BPI_Interact.Interact`
  (params (PlayerActor :type "Actor Object Reference"))
  (set `self.isInteracting` true)
  (if (`self.isUnlocked`)
    (if true :!label _label
      (`/Engine/EditorBlueprintResources/StandardMacros.FlipFlop`
        (:`A`
          (bind (_direction _door_track) (`Timeline|Door Timeline` :!label _label_2)
            (:`Update`
              (`SceneComponent.K2_SetRelativeRotation` (`self.StaticMesh`) (`KismetMathLibrary.MakeRotator` 0.0 0.0 (`KismetMathLibrary.Lerp` 0.0 90.0 _door_track)) false false))))
        (:`B`
          (goto _label_2 :!via `Reverse`))))
    (else
      (message `/Game/BPI_PickUpItem.openInventory` PlayerActor))))

(event `/Game/BPI_SelectItem.ApplyItemToObject`
  (params (selectedItem :type "/Game/W_PickupItem Object Reference"))
  (if (`self.isInteracting`)
    (if (`/Game/W_PickupItem.canOpenLock` selectedItem)
      (set `self.isUnlocked` true)
      (message `/Game/BPI_Door_Unlock.doorUnlocked` self)
      (message `/Game/BPI_PickUpItem.closeInventory` (stale `/Game/BPI_Interact.Interact` PlayerActor))
      (goto _label))))

(fn `UserConstructionScript`)