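; BP_Stove is an interactable stove that the player can switch on and then use with an inventory item, apparently to light a torch.
; Interacting while off, or calling TurnonStove, sets IsOn and reveals the fire effect, which BeginPlay also shows if already on.
; Interacting while on opens the player's inventory; an applied item then gets CanOpenLock, and the player receives light-torch and close-inventory messages.
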(event `/Game/BPI_Interact.Interact`
  (params (PlayerActor :type "Actor Object Reference"))
  (if (`self.isOn`)
    (set `self.isInteracting` true)
    (message `/Game/BPI_PickUpItem.openInventory` PlayerActor)
    (else
      (set `self.isOn` true :!label _label)
      (`SceneComponent.SetHiddenInGame` (`self.FX_Fire`) false false :!label _label_2))))

(event `self.ReceiveBeginPlay`
  (if (`self.isOn`)
    (goto _label_2)))

(event `/Game/BPI_ObjectTrigger.turnOnStove`
  (goto _label))

(event `/Game/BPI_SelectItem.ApplyItemToObject`
  (params (selectedItem :type "/Game/W_PickupItem Object Reference"))
  (if (`self.isInteracting`)
    (set `/Game/W_PickupItem.canOpenLock` true selectedItem)
    (message `/Game/BPI_PickUpItem.lightTorch` (stale `/Game/BPI_Interact.Interact` PlayerActor))
    (message `/Game/BPI_PickUpItem.closeInventory` (stale `/Game/BPI_Interact.Interact` PlayerActor))))

(fn `UserConstructionScript`
  (`parent.UserConstructionScript`))