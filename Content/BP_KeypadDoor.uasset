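; Keypad-locked door actor that swings open and closed once unlocked.
; Interacting while locked flags the door as in use and messages the player to open the keypad menu; DoorUnlocked sets it unlocked and tells the player to close that menu.
; When unlocked, each interaction alternates via FlipFlop between playing and reversing a Timeline that lerps the mesh yaw.
; An unused, disconnected chain that created the keypad widget directly remains, marked for removal.
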(event `/Game/BPI_Interact.Interact`
  (params (PlayerActor :type "Actor Object Reference"))
  (if (`self.isUnlocked`)
    (`/Engine/EditorBlueprintResources/StandardMacros.FlipFlop`
      (:`A`
        (bind (_direction _door_track) (`Timeline|Timeline` :!label _label)
          (:`Update`
            (`SceneComponent.K2_SetRelativeRotation` (`self.StaticMesh`) (`KismetMathLibrary.MakeRotator` 0.0 0.0 (`KismetMathLibrary.Lerp` 0.0 90.0 _door_track)) false false))))
      (:`B`
        (goto _label :!via `Reverse`)))
    (elif (not (`self.isInteracting`))
      (set `self.isInteracting` true)
      (message `/Game/BPI_PickUpItem.openKeypadMenu` PlayerActor))))

(event `/Game/BPI_Door_Unlock.doorUnlocked`
  (set `self.isUnlocked` true)
  (message `/Game/BPI_PickUpItem.closeKeypadMenu` (stale `/Game/BPI_Interact.Interact` PlayerActor)))

(fn `UserConstructionScript`)